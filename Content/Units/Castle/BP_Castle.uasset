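; Castle unit whose death defeats its team.
; On death it casts the game state to PaperGameState, reports the defeat of its team, then runs the parent death logic; a failed cast skips both.
; It supplies a wall material per team, with the arrow material for Neutral, and uses the wall icon as its icon.
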(event `self.Die`
  (bind _aspaper_game_state (cast `PaperGameState` (`GameplayStatics.GetGameState`)))
  (`PaperGameState.Defeat` _aspaper_game_state (`self.Team`))
  (`parent.Die`))

(fn `GetIcon`
  (returns (ReturnValue :type "Texture2D Object Reference"))
  (return "/Game/Units/Wall/T_WallIcon_BC.T_WallIcon_BC"))

(fn `GetMaterial`
  (returns (ReturnValue :type "MaterialInterface Object Reference"))
  (switch `ETeam` (`self.Team`)
    (:`Green`
      (return "/Game/Units/Wall/M_Wall_00.M_Wall_00"))
    (:`Red`
      (return "/Game/Units/Wall/M_Wall_01.M_Wall_01"))
    (:`Purple`
      (return "/Game/Units/Wall/M_Wall_02.M_Wall_02"))
    (:`Brown`
      (return "/Game/Units/Wall/M_Wall_03.M_Wall_03"))
    (:`White`
      (return "/Game/Units/Wall/M_Wall_04.M_Wall_04"))
    (:`Black`
      (return "/Game/Units/Wall/M_Wall_05.M_Wall_05"))
    (:`Neutral`
      (return "/Game/Units/Ground/M_Arrow.M_Arrow"))))

(fn `UserConstructionScript`)