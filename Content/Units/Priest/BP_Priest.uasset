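; Priest unit Blueprint that slowly heals itself and shows a heal effect when it attacks.
; The Passive event calls the parent, then raises HP by one, capped at max HP.
; Attack calls the parent with the victim, then triggers a multicast that spawns the PS_Heal particle emitter attached above the root component on clients.
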(event `self.Passive`
  (`parent.Passive`)
  (`self.SetHP` (`KismetMathLibrary.BMin` (+ (`self.GetHP`) 1) (`self.GetHPMax`))))

(event `self.Attack`
  (params (Victim :type "Unit Object Reference"))
  (`parent.Attack` Victim)
  (`self.Multicast_PlayHealPS`))

(event `Multicast_PlayHealPS`
  (`GameplayStatics.SpawnEmitterAttached` "/Game/Units/Priest/PS_Heal.PS_Heal" (`self.RootComponent`) "Heal PS Emitter" (0.0 0.0 200.0)))

(fn `UserConstructionScript`)