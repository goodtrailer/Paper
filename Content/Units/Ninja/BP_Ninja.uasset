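; Ninja unit Blueprint that extends the parent unit's attack with a reward for killing blows.
; Attack first checks whether Damage exceeds the victim's current HP, then runs the parent attack.
; On a lethal hit it raises Energy to at least EnergyResetThreshold and plays a one-shot kill animation on the skeletal mesh.
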(event `self.Attack`
  (params (Victim :type "Unit Object Reference"))
  (set `self.Lethal` (< (`self.GetHP` Victim) (`KismetMathLibrary.Conv_IntToByte` (`self.Damage`))))
  (`parent.Attack` Victim)
  (if (`self.Lethal`)
    (set `self.Energy` (`KismetMathLibrary.BMax` (`self.Energy`) (`self.EnergyResetThreshold`)))
    (`SkeletalMeshComponent.PlayAnimation` (`self.SkeletalMeshComponent`) (`self.KillAnim`) false)))

(fn `UserConstructionScript`)