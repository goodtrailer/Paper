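; BP_Scout is the Scout unit, which deals bonus damage when attacking Miner-type units.
; Its Attack event temporarily adds BonusMinerDamage to Damage against Miners, calls the parent attack, then restores the original value and multicasts a stomp animation.
; Attacks on other unit types pass straight to the parent attack.
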(event `self.Attack`
  (params (Victim :type "Unit Object Reference"))
  (bind _damage (`self.Damage`))
  (if (== (enumliteral `EType` "Miner") (`Unit.Type` Victim))
    (bind _output_get (set `self.TempDamage` _damage))
    (set `self.Damage` (+ (`self.BonusMinerDamage`) _damage))
    (`parent.Attack` Victim)
    (set `self.Damage` _output_get)
    (`self.Multicast_PlayAnimation` (`self.StompAnim`))
    (else
      (`parent.Attack` Victim))))

(fn `UserConstructionScript`)