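; BP_Knight is the Knight unit Blueprint, supplying the unit's team material, cost and icon.
; GetMaterial switches on Team to pick one of the numbered knight materials, except Neutral, which returns M_Arrow.
; GetCost and GetIcon return a fixed cost and the knight icon texture, and the construction script is empty.
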(fn `GetCost`
  (returns (ReturnValue :type Integer))
  (return 55))

(fn `GetIcon`
  (returns (ReturnValue :type "Texture2D Object Reference"))
  (return "/Game/Units/Knight/T_KnightIcon_BC.T_KnightIcon_BC"))

(fn `GetMaterial`
  (returns (ReturnValue :type "MaterialInterface Object Reference"))
  (switch `ETeam` (`self.Team`)
    (:`Green`
      (return "/Game/Units/Knight/M_Knight_00.M_Knight_00"))
    (:`Red`
      (return "/Game/Units/Knight/M_Knight_01.M_Knight_01"))
    (:`Purple`
      (return "/Game/Units/Knight/M_Knight_02.M_Knight_02"))
    (:`Brown`
      (return "/Game/Units/Knight/M_Knight_03.M_Knight_03"))
    (:`White`
      (return "/Game/Units/Knight/M_Knight_04.M_Knight_04"))
    (:`Black`
      (return "/Game/Units/Knight/M_Knight_05.M_Knight_05"))
    (:`Neutral`
      (return "/Game/Units/Ground/M_Arrow.M_Arrow"))))

(fn `UserConstructionScript`)