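; Miner unit for a grid-based game that earns gold from mines and hits walls harder.
; Its Passive checks the four orthogonal neighbor tiles through PaperGameState, and the first Mine found grants its team bonus income, with the miner turning to face it.
; Attack temporarily adds bonus damage against Wall victims around the parent call, then restores it.
; Mining and wall hits both multicast the mining animation.
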(event `self.Passive`
  (`parent.Passive`)
  (bind _aspaper_game_state (cast `PaperGameState` (`GameplayStatics.GetGameState`)))
  (bind _returnvalue (`self.GetCoordinatesVector`))
  (bind _returnvalue_2 (+ _returnvalue (make `IntPoint` -1)))
  (bind _returnvalue_3 (`PaperGameState.GetUnit` _aspaper_game_state _returnvalue_2))
  (`/Engine/EditorBlueprintResources/StandardMacros.IsValid` _returnvalue_3
    (:`Is Valid`
      (if (== (`Unit.Type` _returnvalue_3) (enumliteral `EType` "Mine"))
        (set `self.MineVector` _returnvalue_2)
        (`PaperGameState.ChangeGold` _aspaper_game_state (`self.Team`) (`self.BonusIncome`) :!label _label)
        (`self.FaceCoordinates` (`self.MineVector`))
        (`self.Multicast_PlayAnimation` (`self.MineAnim`))
        (else
          (bind _returnvalue_4 (+ _returnvalue (make `IntPoint` 1)))
          (bind _returnvalue_5 (`PaperGameState.GetUnit` _aspaper_game_state _returnvalue_4 :!label _label_2))
          (`/Engine/EditorBlueprintResources/StandardMacros.IsValid` _returnvalue_5
            (:`Is Valid`
              (if (== (`Unit.Type` _returnvalue_5) (enumliteral `EType` "Mine"))
                (set `self.MineVector` _returnvalue_4)
                (goto _label)
                (else
                  _)))
            (:`Is Not Valid`
              _))
          (bind _returnvalue_6 (+ _returnvalue (make `IntPoint` 0 -1)))
          (bind _returnvalue_7 (`PaperGameState.GetUnit` _aspaper_game_state _returnvalue_6))
          (`/Engine/EditorBlueprintResources/StandardMacros.IsValid` _returnvalue_7
            (:`Is Valid`
              (if (== (`Unit.Type` _returnvalue_7) (enumliteral `EType` "Mine"))
                (set `self.MineVector` _returnvalue_6)
                (goto _label)
                (else
                  _)))
            (:`Is Not Valid`
              _))
          (bind _returnvalue_8 (+ _returnvalue (make `IntPoint` 0 1)))
          (bind _returnvalue_9 (`PaperGameState.GetUnit` _aspaper_game_state _returnvalue_8))
          (`/Engine/EditorBlueprintResources/StandardMacros.IsValid` _returnvalue_9
            (:`Is Valid`
              (if (== (`Unit.Type` _returnvalue_9) (enumliteral `EType` "Mine"))
                (set `self.MineVector` _returnvalue_8)
                (goto _label)))))))
    (:`Is Not Valid`
      (goto _label_2))))

(event `self.Attack`
  (params (Victim :type "Unit Object Reference"))
  (bind _damage (`self.Damage`))
  (if (== (enumliteral `EType` "Wall") (`Unit.Type` Victim))
    (bind _output_get (set `self.TempDamage` _damage))
    (set `self.Damage` (+ (`self.BonusWallDamage`) _damage))
    (`parent.Attack` Victim)
    (set `self.Damage` _output_get)
    (`self.Multicast_PlayAnimation` (`self.MineAnim`))
    (else
      (`parent.Attack` Victim))))

(fn `UserConstructionScript`)