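; BP_Spawn is the spawn unit Blueprint, supplying its team-dependent material and its icon.
; GetMaterial switches on Team, returning a dedicated spawn material for each colored team and the arrow material for Neutral.
; GetIcon returns the same arrow texture regardless of team, and the construction script is empty.
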(fn `GetIcon`
  (returns (ReturnValue :type "Texture2D Object Reference"))
  (return "/Game/Units/Ground/T_Arrow_BC.T_Arrow_BC"))

(fn `GetMaterial`
  (returns (ReturnValue :type "MaterialInterface Object Reference"))
  (switch `ETeam` (`self.Team`)
    (:`Green`
      (return "/Game/Units/Spawn/M_Spawn_00.M_Spawn_00"))
    (:`Red`
      (return "/Game/Units/Spawn/M_Spawn_01.M_Spawn_01"))
    (:`Purple`
      (return "/Game/Units/Spawn/M_Spawn_02.M_Spawn_02"))
    (:`Brown`
      (return "/Game/Units/Spawn/M_Spawn_03.M_Spawn_03"))
    (:`White`
      (return "/Game/Units/Spawn/M_Spawn_04.M_Spawn_04"))
    (:`Black`
      (return "/Game/Units/Spawn/M_Spawn_05.M_Spawn_05"))
    (:`Neutral`
      (return "/Game/Units/Ground/M_Arrow.M_Arrow"))))

(fn `UserConstructionScript`)