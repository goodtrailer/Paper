(event `self.Build`
  (params (DesiredTeam :type "ETeam Enum" :default "TeamGreen"))
  (bind _staticmeshcomponent (`self.StaticMeshComponent`))
  (`self.BuildMisc` true (make `Cardinal` (`|MakeArray` true true true true)) DesiredTeam)
  (switch `int` (`KismetMathLibrary.RandomInteger` 4)
    (:`0`
      (`StaticMeshComponent.SetStaticMesh` _staticmeshcomponent null))
    (:`1`
      (`StaticMeshComponent.SetStaticMesh` _staticmeshcomponent null))
    (:`2`
      (`StaticMeshComponent.SetStaticMesh` _staticmeshcomponent null))
    (:`3`
      (`StaticMeshComponent.SetStaticMesh` _staticmeshcomponent null))
    (:`4`
      (`StaticMeshComponent.SetStaticMesh` _staticmeshcomponent null))))

(event `self.Die`
  (`self.Multicast_Defeat`)
  (`parent.Die`))

(event `Multicast_Defeat`
  (if (not (`KismetSystemLibrary.IsDedicatedServer`))
    (bind _aspaper_game_instance (cast `PaperGameInstance` (`GameplayStatics.GetGameInstance`)))
    (if (== (`PaperGameInstance.Team` _aspaper_game_instance) (`self.Team`))
      (bind _returnvalue (`|CreateWidget` "/Game/Blueprints/BP_DefeatInterface.BP_DefeatInterface_C" (`GameplayStatics.GetPlayerController` 0)))
      (`/Game/Blueprints/BP_DefeatInterface.Build` _returnvalue false)
      (`UserWidget.AddToViewport` _returnvalue 0))))

(fn `GetIcon`
  (returns (ReturnValue :type "Texture2D Object Reference"))
  (return "/Game/Textures/T_WallIcon_BC.T_WallIcon_BC"))

(fn `GetMaterial`
  (returns (ReturnValue :type "MaterialInterface Object Reference"))
  (switch `ETeam` (`self.Team`)
    (:`TeamGreen`
      (return "/Game/Materials/M_Wall_00.M_Wall_00"))
    (:`TeamRed`
      (return "/Game/Materials/M_Wall_01.M_Wall_01"))
    (:`TeamNeutral`
      (return "/Game/Materials/M_Arrow.M_Arrow"))))

(fn `UserConstructionScript`)