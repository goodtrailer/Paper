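; Player controller Blueprint that shows the end screen when a team wins or is defeated.
; CheckVictory takes the player out of the game on the server and builds an end-screen widget whose variant depends on whether the player's team is the winner, Neutral or another team.
; CheckDefeat does the same with its own variant, but only if the player's team is the defeated one.
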(event `self.CheckVictory`
  (params (WinningTeam :type "ETeam Enum" :default "Green"))
  (`self.Server_SetInGame` false)
  (bind _returnvalue (`|CreateWidget` "/Game/Blueprints/BP_EndScreenGUI.BP_EndScreenGUI_C"))
  (bind _returnvalue_2 (`self.GetPaperPlayerState`))
  (bind _team (`PaperPlayerState.Team` _returnvalue_2))
  (if (== WinningTeam _team)
    (`/Game/Blueprints/BP_EndScreenGUI.Build` _returnvalue 0)
    (elif (== _team (enumliteral `ETeam` "Neutral"))
      (`/Game/Blueprints/BP_EndScreenGUI.Build` _returnvalue 3)
      (else
        (`/Game/Blueprints/BP_EndScreenGUI.Build` _returnvalue 2)))))

(event `self.CheckDefeat`
  (params (DefeatedTeam :type "ETeam Enum" :default "Green"))
  (bind _returnvalue (`self.GetPaperPlayerState`))
  (if (== (`PaperPlayerState.Team` _returnvalue) DefeatedTeam)
    (`self.Server_SetInGame` false)
    (bind _returnvalue_2 (`|CreateWidget` "/Game/Blueprints/BP_EndScreenGUI.BP_EndScreenGUI_C" (`GameplayStatics.GetPlayerController` 0)))
    (`/Game/Blueprints/BP_EndScreenGUI.Build` _returnvalue_2 1)))

(fn `UserConstructionScript`)