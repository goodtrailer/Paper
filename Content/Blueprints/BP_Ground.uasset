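; BP_Ground is a ground piece that marks its collidable directions with arrow meshes when built for a team.
; Its Build event passes the BIsCollidable direction flags and the Team to BuildMisc.
; It then checks the four directions and, for each one set, adds a scaled, raised arrow static mesh component at runtime, yawed in quarter turns by index.
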(event `self.Build`
  (params (team :type "ETeam Enum" :default "TeamGreen"))
  (`self.BuildMisc` (`.Directions` (break `Cardinal` (`self.bIsCollidable`))) team)
  (for _index (range 4)
    (if (`|GetArrayItem` (`.Directions` (break `Cardinal` (`self.bIsCollidable`))) _index)
      (bind _returnvalue (`AddComponent|NODE_AddStaticMeshComponent-1` :`RelativeTransform` (`KismetMathLibrary.MakeTransform` (0.0 0.0 100.0) (`KismetMathLibrary.MakeRotator` 0.0 0.0 (* _index 90.0)) (100.0 100.0 100.0))))
      (`StaticMeshComponent.SetStaticMesh` _returnvalue "/Game/Meshes/SM_Arrow.SM_Arrow")
      (`PrimitiveComponent.SetMaterial` _returnvalue 0 "/Game/Materials/M_Arrow.M_Arrow"))))

(fn `UserConstructionScript`)