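; BP_Miner is a grid-based unit that earns gold for its team and deals extra damage to walls.
; Its Passive runs the parent logic, then checks the four orthogonal neighbors via PaperGameState and grants bonus income once if any is a Mine.
; Attack temporarily raises Damage against Wall victims before calling the parent attack.
; Overrides supply its cost, icon and team-specific material.
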(event `self.Passive`
  (`parent.Passive`)
  (bind _aspaper_game_state (cast `PaperGameState` (`GameplayStatics.GetGameState`)))
  (bind _returnvalue (`self.GetCoordinatesVector`))
  (bind _returnvalue_2 (`PaperGameState.GetUnit` _aspaper_game_state (+ _returnvalue (make `IntPoint` -1))))
  (`/Engine/EditorBlueprintResources/StandardMacros.IsValid` _returnvalue_2
    (:`Is Valid`
      (if (== (`Unit.Type` _returnvalue_2) (enumliteral `EType` "Mine"))
        (`PaperGameState.ChangeGold` _aspaper_game_state (`self.Team`) (`self.BonusIncome`))
        (else
          (bind _returnvalue_3 (`PaperGameState.GetUnit` _aspaper_game_state (+ _returnvalue (make `IntPoint` 1)) :!label _label))
          (`/Engine/EditorBlueprintResources/StandardMacros.IsValid` _returnvalue_3
            (:`Is Valid`
              (if (== (`Unit.Type` _returnvalue_3) (enumliteral `EType` "Mine"))
                (`PaperGameState.ChangeGold` _aspaper_game_state (`self.Team`) (`self.BonusIncome`))
                (else
                  (bind _returnvalue_4 (`PaperGameState.GetUnit` _aspaper_game_state (+ _returnvalue (make `IntPoint` 0 -1)) :!label _label_2))
                  (`/Engine/EditorBlueprintResources/StandardMacros.IsValid` _returnvalue_4
                    (:`Is Valid`
                      (if (== (`Unit.Type` _returnvalue_4) (enumliteral `EType` "Mine"))
                        (`PaperGameState.ChangeGold` _aspaper_game_state (`self.Team`) (`self.BonusIncome`))
                        (else
                          (bind _returnvalue_5 (`PaperGameState.GetUnit` _aspaper_game_state (+ _returnvalue (make `IntPoint` 0 1)) :!label _label_3))
                          (`/Engine/EditorBlueprintResources/StandardMacros.IsValid` _returnvalue_5
                            (:`Is Valid`
                              (if (== (`Unit.Type` _returnvalue_5) (enumliteral `EType` "Mine"))
                                (`PaperGameState.ChangeGold` _aspaper_game_state (`self.Team`) (`self.BonusIncome`))))))))
                    (:`Is Not Valid`
                      (goto _label_3))))))
            (:`Is Not Valid`
              (goto _label_2))))))
    (:`Is Not Valid`
      (goto _label))))

(event `self.Attack`
  (params (Victim :type "Unit Object Reference"))
  (bind _damage (`self.Damage`))
  (if (== (enumliteral `EType` "Wall") (`Unit.Type` Victim))
    (bind _output_get (set `self.TempDamage` _damage))
    (set `self.Damage` (+ (`self.BonusWallDamage`) _damage))
    (`parent.Attack` Victim)
    (set `self.Damage` _output_get)
    (else
      (`parent.Attack` Victim))))

(fn `GetCost`
  (returns (ReturnValue :type Integer))
  (return 25))

(fn `GetIcon`
  (returns (ReturnValue :type "Texture2D Object Reference"))
  (return "/Game/Textures/T_Arrow_BC.T_Arrow_BC"))

(fn `GetMaterial`
  (returns (ReturnValue :type "MaterialInterface Object Reference"))
  (switch `ETeam` (`self.Team`)
    (:`Green`
      (return "/Game/Materials/M_Miner_00.M_Miner_00"))
    (:`Red`
      (return "/Game/Materials/M_Miner_01.M_Miner_01"))
    (:`Purple`
      (return "/Game/Materials/M_Miner_02.M_Miner_02"))
    (:`Brown`
      (return "/Game/Materials/M_Miner_03.M_Miner_03"))
    (:`White`
      (return "/Game/Materials/M_Miner_04.M_Miner_04"))
    (:`Black`
      (return "/Game/Materials/M_Miner_05.M_Miner_05"))
    (:`Neutral`
      (return "/Game/Materials/M_Arrow.M_Arrow"))))

(fn `UserConstructionScript`)