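; Unit actor for a team-based game, with hit points, a targetable flag and per-side collision flags.
; The Build event takes a team and passes fixed unit defaults to BuildMisc, making it targetable and collidable on all four sides.
; BuildMisc stores these values, blocks a custom trace channel on the mesh and picks a material by team.
; All three team materials are currently the same arrow material.
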(event `self.Build`
  (params (team :type "ETeam Enum" :default "TeamGreen"))
  (`self.BuildMisc` "TypeUnit" 5 5 true (`|MakeArray` true true true true) team "/Game/Materials/M_Arrow.M_Arrow" "/Game/Materials/M_Arrow.M_Arrow" "/Game/Materials/M_Arrow.M_Arrow"))

(fn `BuildMisc`
  (params (Type :type "EType Enum" :default "TypeUnit") (`Max HP` :type Byte) (`Starting HP` :type Byte) (`Is Targetable` :type Boolean) (`Collidable (URDL)` :type "Array of Boolean") (Team :type "ETeam Enum" :default "TeamGreen") (`Green Material` :type "MaterialInterface Object Reference") (`Red Material` :type "MaterialInterface Object Reference") (`Neutral Material` :type "MaterialInterface Object Reference"))
  (bind _staticmesh (`self.StaticMesh`))
  (set `self.Type` Type)
  (set `self.HPMax` `Max HP`)
  (set `self.HP` `Starting HP`)
  (set `self.bIsTargetable` `Is Targetable`)
  (`PrimitiveComponent.SetCollisionResponseToChannel` (`self.StaticMesh`) "ECC_GameTraceChannel1" "ECR_Block")
  (set `self.bIsCollidable` (make `Cardinal` `Collidable (URDL)`))
  (bind _output_get (set `self.Team` Team))
  (switch `ETeam` _output_get
    (:`TeamGreen`
      (`PrimitiveComponent.SetMaterial` _staticmesh 0 `Green Material`))
    (:`TeamRed`
      (`PrimitiveComponent.SetMaterial` _staticmesh 0 `Red Material`))
    (:`TeamNeutral`
      (`PrimitiveComponent.SetMaterial` _staticmesh 0 `Neutral Material`))))

(fn `UserConstructionScript`
  (`self.SetActorTickEnabled` true))